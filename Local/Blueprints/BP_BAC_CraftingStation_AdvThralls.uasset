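; Interactable component for crafting stations with artisan thrall slots that toggles the crafting GUI for the player using it.
; Activation or deselection sets or clears the character's interacting actor and tracks that player.
; On BeginPlay it loads the owner's saved inventory through its persistence component IDs and binds to the CraftingQueue's artisan slot signal.
; A valid thrall in that slot grants the tracked player the exceptional-crafting achievement via AchievementInterface.
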(event `InteractableInterface.InteractableSelectionChanged`
  (params (IsSelected :type Boolean) (Instigator :type "PlayerController Object Reference") (InstanceIndex :type Integer))
  (if (and (not IsSelected) (`self.IsOpen`))
    (set `self.IsOpen` false :!label _label)
    (`ConanCharacter.SetInteractingActor` (cast `ConanCharacter` (`Controller.K2_GetPawn` (stale `InteractableInterface.InteractableActivate` Instigator)) :!pure true) null "None")
    (set `self.InteractingPlayer` null)))

(event `InteractableInterface.InteractableActivate`
  (params (Component :type "PrimitiveComponent Object Reference") (Instigator :type "PlayerController Object Reference") (HitIndex :type Integer) (TriggeredFromRadialWheel :type Boolean))
  (bind _asconan_character (cast `ConanCharacter` (`Controller.K2_GetPawn` Instigator) :!pure true))
  (if (`self.IsOpen`)
    (goto _label)
    (else
      (set `self.IsOpen` true)
      (`ConanCharacter.SetInteractingActor` _asconan_character (`self.GetOwner`) "CraftingGUI")
      (set `self.InteractingPlayer` _asconan_character))))

(event `self.ReceiveBeginPlay`
  (bind _returnvalue (`self.GetOwner`))
  (`parent.ReceiveBeginPlay`)
  (for _array_element (`Actor.K2_GetComponentsByClass` _returnvalue "/Script/ConanSandbox.ConanBuildingPersistenceComponent")
    (bind (_uid _result) (`LoadInventoryCallProxy.LoadInventory` (`PersistenceComponent.GetUniqueID` _array_element))
      (:`OnSuccess`
        (`LoadInventoryCallProxy.ProcessInventoryData` (`self.GetOwner`) _result))))
  (add `CraftingQueue.SignalArtisanSlotChanged` (`Actor.GetComponentByClass` _returnvalue "/Script/ConanSandbox.CraftingQueue") (delegate `GiveAchievement`)))

(event `self.ReceiveEndPlay`
  (params (EndPlayReason :type "EEndPlayReason Enum" :default "Destroyed"))
  (`parent.ReceiveEndPlay` EndPlayReason)
  (remove `CraftingQueue.SignalArtisanSlotChanged` (`Actor.GetComponentByClass` (`self.GetOwner`) "/Script/ConanSandbox.CraftingQueue") (delegate `GiveAchievement`)))

(event `GiveAchievement`
  (params (thrallItem :type "ThrallItem Object Reference"))
  (if (`KismetSystemLibrary.IsValid` thrallItem)
    (bind _asachievement_interface (cast `/Game/Systems/Achievements/AchievementInterface` (`Actor.GetComponentByInterface` (`Pawn.GetController` (`self.InteractingPlayer`)) "/Game/Systems/Achievements/AchievementInterface.AchievementInterface_C")))
    (`/Game/Systems/Achievements/AchievementInterface.GiveAchievementProgressInterfaceFunc` _asachievement_interface "ACH_CraftExceptional" 100.0 0)))